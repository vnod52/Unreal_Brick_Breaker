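; Player blueprint for a paddle-and-ball game that moves the paddle and launches the ball.
; Horizontal axis input pushes the Paddle with an impulse scaled by Speed.
; On BeginPlay, and through the SpawnNewBall event, a Ball spawns at the Arrow component's transform and is stored.
; The Fire action launches the stored ball along the Arrow's forward vector if it is valid and not yet active.
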(event `InputAxis|MoveHorizontal`
  (params (AxisValue :type "Float (single-precision)"))
  ;[1 1 1] Movement
  (`PrimitiveComponent.AddImpulse` (`self.Paddle`) (`KismetMathLibrary.MakeVector` (* AxisValue (`self.Speed`))) "None" false))

(event `self.ReceiveBeginPlay`
  (`self.Spawn New Ball`))

(event `Spawn New Ball`
  ;[1 1 1] Spawn new ball
  (bind _returnvalue (`|SpawnActorFromClass` "/Game/Blueprints/Ball.Ball_C" (`SceneComponent.K2_GetComponentToWorld` (`self.Arrow`)) "AlwaysSpawn" "OverrideRootScale" null null))
  (set `self.Ball` _returnvalue))

(event `InputAction|Fire`
  (params (Key :type "Key Structure"))
  (bind _ball (`self.Ball`))
  ;[1 1 1] Launch Ball
  (:`Pressed`
    (if (and (`KismetSystemLibrary.IsValid` _ball) (not (`/Game/Blueprints/Ball.Active` _ball)))
      (`/Game/Blueprints/Ball.Launch` _ball (`KismetMathLibrary.Conv_RotatorToVector` (`SceneComponent.K2_GetComponentRotation` (`self.Arrow`)))))))

(fn `UserConstructionScript`)