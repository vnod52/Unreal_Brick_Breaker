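; Ball actor for a paddle game, launched by impulse and kept at a fixed speed on diagonal headings.
; Until launched, it follows the Player's Arrow component every tick.
; Each tick also clamps velocity to Speed, snapping yaw to 90-degree steps offset by 45 degrees via a rotate, round, unrotate trick.
; When destroyed, it reports the lost ball to MyGameMode and asks the Player to spawn a new one.
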(event Custom|Launch
  (params (Direction :type Vector))
  ;[1 1 1] Launch ball
  (Variables|Default|SetActive true)
  (Physics|AddImpulse (Variables|Default|GetBall) Direction "None" true))

(event Custom|Clamp%20Velocity
  (bind _returnvalue (Transformation|GetVelocity))
  (bind _returnvalue_2 (Math|Rotator|MakeRotator 0.0 0.0 45.0))
  (bind _speed (Variables|Default|Getspeed))
  (bind _returnvalue_3 (Math|Vector|ClampVectorSize _returnvalue _speed _speed))
  ;[1 1 1] Clamp ball velocity
  (Physics|SetPhysicsLinearVelocity (Variables|Default|GetBall) (* (Math|Vector|UnrotateVector (Math|Rotator|GetRotationXVector (Math|Rotator|MakeRotator 0.0 0.0 (|((round((A/B)))*B) (.yaw (Math|Rotator|MakeRotfromX (Math|Vector|RotateVector _returnvalue_3 _returnvalue_2))) 9e+01))) _returnvalue_2) (Math|Vector|VectorLength _returnvalue_3)) false "None"))

(event Custom|Update%20Position
  ;[1 1 1] Attach to paddle while not active
  (if (not (Variables|Default|GetActive))
    (Transformation|SetActorLocation (Transformation|GetWorldLocation (Variables|/Game/Blueprints/Player.Player_C|GetArrow (Variables|Default|Getplayer))) false false)))

(event EventBeginPlay
  ;[1 1 1] Get Player
  (bind _asplayer (Utilities|Casting|CastToPlayer (Pawn|GetControlledPawn (Game|GetPlayerController 0))))
  (Variables|Default|Setplayer _asplayer)
  ;[1 1 1] Get Game Mode
  (bind _asmy_game_mode (Utilities|Casting|CastToMyGameMode (Game|GetGameMode)))
  (Variables|Default|SetGameMode _asmy_game_mode))

(event EventDestroyed
  ;[1 1 1] Spawn new ball when one is destroyed
  (Default|LostBall (Variables|Default|GetGameMode))
  (Default|SpawnNewBall (Variables|Default|Getplayer)))

(event EventTick
  (params (DeltaSeconds :type Float%20%28single-precision%29))
  (CallFunction|UpdatePosition)
  (CallFunction|ClampVelocity))

(fn ConstructionScript)