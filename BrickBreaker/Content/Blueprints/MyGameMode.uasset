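; Game mode that tracks score and remaining balls and mirrors both to an on-screen GUI widget.
; On BeginPlay it creates the GUI, adds it to the viewport and runs ResetGame, which restores balls to MaxLifes and zeroes the score.
; UpdateScore adds points, clamps the total at zero and pushes it to the GUI.
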(event `self.ReceiveBeginPlay`
  ;[1 1 1] Add GUI
  (bind _returnvalue (`|CreateWidget` "/Game/Blueprints/GUI.GUI_C"))
  (bind _output_get (set `self.GUI` _returnvalue))
  (`UserWidget.AddToViewport` _output_get 0)
  (`self.ResetGame`))

(event `ResetGame`
  (bind _maxlifes (`self.MaxLifes`))
  (bind _gui (`self.GUI`))
  (set `self.CurrentBalls` _maxlifes)
  (set `/Game/Blueprints/GUI.Balls Left` _maxlifes _gui)
  (set `/Game/Blueprints/GUI.Score` 0.0 _gui)
  (set `self.CurrentScore` 0.0))

(event `UpdateScore`
  (params (Points :type "Float (double-precision)"))
  (bind _returnvalue (+ Points (`self.CurrentScore`)))
  ;[1 1 1] Update Score
  (if (< _returnvalue 0.0)
    (set `self.CurrentScore` 0.0)
    (else
      (set `self.CurrentScore` _returnvalue)))
  (set `/Game/Blueprints/GUI.Score` (`self.CurrentScore`) (`self.GUI`)))

(fn `UserConstructionScript`)